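; BP_Lever is a dungeon lever actor that switches between on and off states and animates its handle.
; ToggleLever flips IsOn through SetLeverState, which stores the state and notifies the BooleanInstigator via CallOnToggle.
; The LeverPull timeline plays when on and reverses when off, driving the LeverHandle's relative roll.
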(event Custom|SetLeverState
  (params (IsActive :type Boolean))
  (bind _output_get (Variables|Default|SetisOn IsActive))
  (Default|CallOnToggle (Variables|Default|GetBooleanInstigator))
  (if _output_get
    (bind _x_rotation (Timeline|LeverPull Play)
      (:Update
        (Transformation|SetRelativeRotation (Variables|Default|GetLeverHandle) (Math|Rotator|MakeRotator _x_rotation 0.0 0.0) false false)))
    (else
      (Timeline|LeverPull Reverse))))

(event Custom|ToggleLever
  (CallFunction|SetLeverState (not (Variables|Default|GetisOn))))

(event EventBeginPlay)

(event Collision|EventActorBeginOverlap
  (params (OtherActor :type Actor%20Object%20Reference)))

(event EventTick
  (params (DeltaSeconds :type Float%20%28single-precision%29)))

(fn ConstructionScript)